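; BP_WinTrigger is a level-exit trigger that completes the level when the player overlaps it with no crystals left.
; On overlap it checks for a player and scans the world for any remaining BP_Crystal actors.
; Completion looks up the current level's name in an ordered Levels array and opens the next entry, wrapping to the first level after the last.
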(event `self.ReceiveActorBeginOverlap`
  (params (OtherActor :type "Actor Object Reference"))
  (`/Game/Blueprints/Libraries/CC_MacroLibrary.IsPlayer` OtherActor
    (:`Is Player`
      (if (not (`self.AnyCrystalRemaining`))
        (`self.CompleteLevel`)))))

(fn `AnyCrystalRemaining`
  (returns (ReturnValue :type Boolean))
  (bind _outactors (`GameplayStatics.GetAllActorsOfClass` "/Game/Blueprints/Actors/Collectables/BP_Crystal.BP_Crystal_C"))
  (return (> (`KismetArrayLibrary.Array_Length` _outactors) 0)))

(fn `CompleteLevel`
  (if (`self.IsFinalLevel`)
    (`self.OpenFirstLevel`)
    (else
      (`self.LoadNextLevel`))))

(fn `GetCurrentLevelIndex`
  (returns (`Return Value` :type Integer))
  (bind _returnvalue (`GameplayStatics.GetCurrentLevelName` true))
  (return (`KismetArrayLibrary.Array_Find` (`self.Levels`) (`KismetStringLibrary.Conv_StringToName` _returnvalue))))

(fn `GetNextLevelName`
  (returns (Output :type Name))
  (return (`|GetArrayItem` (`self.Levels`) (+ (`self.GetCurrentLevelIndex`) 1))))

(fn `IsFinalLevel`
  (returns (`Return Value` :type Boolean))
  (return (== (`KismetArrayLibrary.Array_LastIndex` (`self.Levels`)) (`self.GetCurrentLevelIndex`))))

(fn `LoadNextLevel`
  (`GameplayStatics.OpenLevel` (`self.GetNextLevelName`)))

(fn `OpenFirstLevel`
  (`GameplayStatics.OpenLevel` (`|GetArrayItem` (`self.Levels`))))

(fn `UserConstructionScript`)